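; BP_Special is a token piece Blueprint that adds the shared move rule for special pieces on a board.
; HighlightSpecialSquare offsets the piece's X and Y by given increments and highlights that square in the piece's Color if it passes IsValidMoveForSpecial.
; That check queries the game mode's GetOccupant and accepts only valid, unoccupied squares, so occupied squares are never targets.
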(fn `HighlightSpecialSquare`
  (params (XIncr :type Integer) (YIncr :type Integer))
  (locals (TempX :type Integer) (TempY :type Integer))
  (set `local.TempX` (+ (`self.X`) XIncr))
  (set `local.TempY` (+ (`self.Y`) YIncr))
  (if (`self.IsValidMoveForSpecial` (`local.TempX`) (`local.TempY`))
    (`self.HighlightPotentialSquare` (`local.TempX`) (`local.TempY`) (`self.Color`))))

(fn `IsValidMoveForSpecial`
  (params (X :type Integer) (Y :type Integer))
  (returns (IsValidMove :type Boolean))
  (bind (_tokenpiece _isoccupied _isoccupiedbyfriend _isvalid) (`/Game/Divinum/Blueprints/BP_Gamemode.GetOccupant` (`self.GameModeRef`) X Y (`self.Color`)))
  (if _isvalid
    (if _isoccupied
      (return false)
      (else
        (return true)))
    (else
      (return false))))

(fn `UserConstructionScript`
  (`parent.UserConstructionScript`))