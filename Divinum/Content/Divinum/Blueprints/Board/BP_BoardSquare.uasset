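; BP_BoardSquare is one square of a board game, with a light or dark material, a letter-number notation built from its coordinates, and an optional occupant.
; Initialize caches the player controller and game mode, sets the notation, and binds ResetSquare to the board's reset-all event.
; Highlight, select and reset functions set state flags, then SetMarkerColor derives the marker's visibility and material, showing occupied highlighted squares as attackable unless selected.
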(event `InitEvent`
  (`/Engine/EditorBlueprintResources/StandardMacros.IsValid` (`self.BoardRef`)
    (:`Is Valid`
      (add `/Game/Divinum/Blueprints/Board/BP_Board.ResetAllSquares` (`self.BoardRef`) (delegate `ResetSquare`)))))

(event `ResetSquare`
  (`self.ResetMarker`))

(fn `GetLocation`
  (returns (Location :type "Vector Structure"))
  (return (`SceneComponent.K2_GetComponentLocation` (`self.Billboard`))))

(fn `GetYValue`
  (returns (Yvalue :type String))
  (switch `int` (`self.Y`)
    (:`1`
      (return "a"))
    (:`2`
      (return "b"))
    (:`3`
      (return "c"))
    (:`4`
      (return "d"))
    (:`5`
      (return "e"))
    (:`6`
      (return "f"))
    (:`7`
      (return "g"))
    (:`8`
      (return "h"))
    (:`9`
      (return "i"))
    (:`10`
      (return "j"))))

(fn `HasOccupant`
  (returns (HasOccupant :type Boolean))
  (return (`KismetSystemLibrary.IsValid` (`self.OccupantRef`))))

(fn `HighlightMarker`
  (`|ExecutionSequence`
    (:`then_0`
      (set `self.IsHighlighted` true)
      (set `self.IsSelected` false)
      (set `self.IsAttackable` false)
      (set `self.IsTokenPieceSelected` false))
    (:`then_1`
      (if (`self.HasOccupant`)
        (set `self.IsAttackable` true))
      (`self.SetMarkerColor`))))

(fn `Initialize`
  (`self.SetPlayerControllerRef`)
  (`self.Set Game Mode Ref`)
  (`self.SetNotation`)
  (`self.InitEvent`))

(fn `ResetMarker`
  (`|ExecutionSequence`
    (:`then_0`
      (set `self.IsSelected` false)
      (set `self.IsHighlighted` false)
      (set `self.IsAttackable` false)
      (set `self.IsVisible` false)
      (set `self.IsTokenPieceSelected` false))
    (:`then_1`
      (`self.SetMarkerColor`))))

(fn `SelectMarker`
  (if (`self.IsHighlighted`)
    (set `self.IsSelected` true)
    (`self.SetMarkerColor`)))

(fn `Set Game Mode Ref`
  (`/Engine/EditorBlueprintResources/StandardMacros.IsValid` (`self.GamemodeRef`)
    (:`Is Not Valid`
      (bind _asbp_gamemode (cast `/Game/Divinum/Blueprints/BP_Gamemode` (`GameplayStatics.GetGameMode`)))
      (set `self.GamemodeRef` _asbp_gamemode))))

(fn `SetMarkerColor`
  (if (`self.IsHighlighted`)
    (if (`self.IsSelected`)
      (set `self.IsVisible` true)
      (set `self.ActiveMaterial` (`self.SelectMaterial`))
      (elif (`self.IsAttackable`)
        (set `self.IsVisible` true)
        (set `self.ActiveMaterial` (`self.AttackMaterial`))
        (else
          (set `self.IsVisible` true)
          (set `self.ActiveMaterial` (`self.HighlightMaterial`)))))
    (elif (`self.IsTokenPieceSelected`)
      (set `self.IsVisible` true)
      (set `self.ActiveMaterial` (`self.TokenPieceMaterial`))
      (else
        (set `self.IsVisible` false)
        (set `self.ActiveMaterial` (`self.HighlightMaterial`)))))
  (`PrimitiveComponent.SetMaterial` (`self.Marker`) 0 (`self.ActiveMaterial`))
  (`SceneComponent.SetVisibility` (`self.Marker`) (`self.IsVisible`) false))

(fn `SetNotation`
  (set `self.Notation` (`KismetStringLibrary.Concat_StrStr` (`self.GetYValue`) (`KismetStringLibrary.Conv_IntToString` (`self.X`)))))

(fn `SetPlayerControllerRef`
  (`/Engine/EditorBlueprintResources/StandardMacros.IsValid` (`self.PlayerControllerRed`)
    (:`Is Not Valid`
      (bind _asbp_player_controller (cast `/Game/Divinum/Blueprints/BP_PlayerController` (`GameplayStatics.GetPlayerController` 0)))
      (set `self.PlayerControllerRed` _asbp_player_controller))))

(fn `SetSquareColor`
  (bind _square (`self.Square`))
  (switch `/Game/Divinum/Blueprints/En_Color` (`self.Color`)
    (:`NewEnumerator0`
      (`PrimitiveComponent.SetMaterial` _square 0 (`self.LightColor`)))
    (:`NewEnumerator1`
      (`PrimitiveComponent.SetMaterial` _square 0 (`self.DarkColor`)))))

(fn `UnhighlightMarker`
  (`|ExecutionSequence`
    (:`then_0`
      (set `self.IsAttackable` false)
      (set `self.IsHighlighted` false)
      (set `self.IsSelected` false))
    (:`then_1`
      (`self.SetMarkerColor`))))

(fn `UnselecteMarker`
  (set `self.IsSelected` false)
  (`self.SetMarkerColor`))

(fn `UserConstructionScript`
  (`self.SetSquareColor`))