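; Player controller for a two-player token board game that handles player input and the main HUD.
; It caches the game mode and forwards the move-token action and camera rotation axis to it.
; It creates the main UI widget and refreshes it from game mode state: active player, both players' names and captures, move count, a stored message and game-over status.
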(event `self.ReceiveBeginPlay`
  (`self.SetGameModeRef`))

(event `InputAction|MoveTokenPiece`
  (params (Key :type "Key Structure"))
  (:`Pressed`
    (`/Game/Divinum/Blueprints/BP_Gamemode.ProcessMove` (`self.GameModeRef`))))

(event `InputAxis|RotatePlayerCamera`
  (params (AxisValue :type "Float (single-precision)"))
  (`/Game/Divinum/Blueprints/BP_Gamemode.RotateCamera` (`self.GameModeRef`) AxisValue))

(fn `Initialize`
  (`self.SetGameModeRef`))

(fn `SetGameModeRef`
  (`/Engine/EditorBlueprintResources/StandardMacros.IsValid` (`self.GameModeRef`)
    (:`Is Not Valid`
      (bind _asbp_gamemode (cast `/Game/Divinum/Blueprints/BP_Gamemode` (`GameplayStatics.GetGameMode`)))
      (set `self.GameModeRef` _asbp_gamemode))))

(fn `SetMainUI`
  (bind _returnvalue (`|CreateWidget` "/Game/Divinum/UI/UI_Main.UI_Main_C" self))
  (bind _output_get (set `self.MainUIRef` _returnvalue))
  (`UserWidget.AddToViewport` _output_get 0)
  (`/Game/Divinum/UI/UI_Main.OpenUI` (`self.MainUIRef`))
  (`self.UpdateUI`))

(fn `SetMessage`
  (params (NewMessage :type String))
  (set `self.Message` NewMessage))

(fn `SetPlayerInfoInUI`
  (params (PlayerIndex :type Integer))
  (bind (_name _color _index _haslegalmovesflag _movecount _captures) (break `/Game/Divinum/Blueprints/ST_Player` (`/Game/Divinum/Blueprints/BP_Gamemode.GetPlayerByIndex` (`self.GameModeRef`) PlayerIndex)))
  (`/Game/Divinum/UI/UI_Main.SetPlayerName` (`self.MainUIRef`) _color _name)
  (`/Game/Divinum/UI/UI_Main.SetCaptureCount` (`self.MainUIRef`) _color _captures))

(fn `UpdateUI`
  (`/Game/Divinum/UI/UI_Main.SetActivePlayer` (`self.MainUIRef`) (`/Game/Divinum/Blueprints/BP_Gamemode.GetActivePlayerColor` (`self.GameModeRef`)))
  (`|ExecutionSequence`
    (:`then_0`
      (`self.SetPlayerInfoInUI` 0)
      (`self.SetPlayerInfoInUI` 1))
    (:`then_1`
      (`/Game/Divinum/UI/UI_Main.SetMoveCount` (`self.MainUIRef`) (`/Game/Divinum/Blueprints/BP_Gamemode.GetMoveCount` (`self.GameModeRef`)))
      (`/Game/Divinum/UI/UI_Main.SetMessage1` (`self.MainUIRef`) (`self.Message`))
      (if (`/Game/Divinum/Blueprints/BP_Gamemode.GetGameStatus` (`self.GameModeRef`))
        (`/Game/Divinum/UI/UI_Main.SetMessage2` (`self.MainUIRef`) "Game Over")
        (else
          (`/Game/Divinum/UI/UI_Main.SetMessage2` (`self.MainUIRef`) "Good Move!"))))))

(fn `UserConstructionScript`)